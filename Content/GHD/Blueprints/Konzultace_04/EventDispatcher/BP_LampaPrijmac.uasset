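; BP_LampaPrijmac is a lamp that dims its spot light as the player character moves away from it, demonstrating an event dispatcher subscriber.
; On BeginPlay it casts the player character to ThirdPersonCharacter and binds to its OnCharacterPosition dispatcher.
; Each broadcast supplies the player position, whose distance to the lamp is mapped through a clamped range and scaled to set the light intensity, with no Tick in the lamp.
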(event `self.ReceiveBeginPlay`
  (bind _asthird_person_character (cast `/Game/ThirdPersonBP/Blueprints/ThirdPersonCharacter` (`GameplayStatics.GetPlayerCharacter` 0))) ; Zjisti hráče.
  (add `/Game/ThirdPersonBP/Blueprints/ThirdPersonCharacter.OnCharacterPosition` _asthird_person_character (delegate `Pozice`)) ; Nabinduj (Subscription) pro event
)

(event `Pozice`
  (params (PoziceHrace :type "Vector Structure"))
  (`LightComponent.SetIntensity` (`self.SpotLight`) (* (`KismetMathLibrary.MapRangeClamped` (`KismetMathLibrary.Vector_Distance` PoziceHrace (`self.K2_GetActorLocation` self)) 100.0 500.0 1.0) 20000.0)))

(fn `UserConstructionScript`)