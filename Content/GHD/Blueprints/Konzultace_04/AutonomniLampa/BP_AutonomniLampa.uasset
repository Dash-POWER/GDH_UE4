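; Autonomous lamp actor whose spot light brightens as the player character approaches and dims as they move away.
; On BeginPlay it caches the player's ThirdPersonCharacter and starts a looping short-interval timer instead of using Tick.
; Each timer call checks that the character is valid, then maps its clamped distance from the lamp to the spot light's intensity.
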(event `self.ReceiveBeginPlay`
  ;[0 0 0] Zjisti hráče ze světa a ulož referenci do proměné.
  (bind _asthird_person_character (cast `/Game/ThirdPersonBP/Blueprints/ThirdPersonCharacter` (`GameplayStatics.GetPlayerCharacter` 0)))
  (set `self.As Third Person Character` _asthird_person_character)
  (`KismetSystemLibrary.K2_SetTimerDelegate` (delegate `MyEvent`) 0.1 true) ; Vlastní časovač
)

(event `MyEvent`
  (`self.As Third Person Character` ; Je charakter validní (Existuje?)
    (:`then`
      (`LightComponent.SetIntensity` (`self.SpotLight`) (* (`KismetMathLibrary.MapRangeClamped` (`KismetMathLibrary.Vector_Distance` (`self.K2_GetActorLocation` (`self.As Third Person Character`)) (`self.K2_GetActorLocation` self)) 100.0 500.0 1.0) 20000.0)) ; Nastav intensitu.
    )
    (:`else`)))

(fn `UserConstructionScript`)