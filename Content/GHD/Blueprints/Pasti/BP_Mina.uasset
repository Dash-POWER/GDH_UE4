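; BP_Mina is a one-shot landmine trap, a child of BP_ObecnaPast that overrides its Aktivace event.
; Construction applies the configurable blast strength and effect to the radial force and particle components.
; The first activation swaps the mesh for a decal and plays the particles.
; Only if the character's Health is depleted does it ragdoll them, fire the impulse, replace the HUD with Game Over and call parent Aktivace.
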(fn `Aktivace`
  (params (Character :type "/Game/ThirdPersonBP/Blueprints/ThirdPersonCharacter Object Reference"))
  (locals (TheCharacter :type "/Game/ThirdPersonBP/Blueprints/ThirdPersonCharacter Object Reference"))
  (bind _thecharacter (`local.TheCharacter`))
  ;[0 0 0] Když nám řekne parent (BP_ObecnaPast), že někdo prošel, tady už definujeme, co se přesně stane.
  ; (Tady přepíšeme původní funkci "Aktivace" na něco vlastního, třeba explozi. Když už jsme v BP_Mina)
  (set `local.TheCharacter` Character)
  (if (not (`self.IsExploded`))
    (set `self.IsExploded` true)
    (`SceneComponent.SetVisibility` (`self.Decal`) true false)
    (`ActorComponent.Activate` (`self.Particle`) false)
    (`SceneComponent.SetVisibility` (`self.StaticMesh`) false false)
    (if (<= (`/Game/ThirdPersonBP/Blueprints/ThirdPersonCharacter.Health` (`local.TheCharacter`)) 0)
      (`PrimitiveComponent.SetSimulatePhysics` (`Character.Mesh` _thecharacter) true)
      (`CharacterMovementComponent.DisableMovement` (`Character.CharacterMovement` _thecharacter))
      (`RadialForceComponent.FireImpulse` (`self.RadialForce`))
      (bind _returnvalue (`|CreateWidget` "/Game/GHD/Widgets/UMG_GameOver.UMG_GameOver_C"))
      (`UserWidget.AddToViewport` _returnvalue 0)
      (`Widget.RemoveFromParent` (`/Game/ThirdPersonBP/Blueprints/ThirdPersonCharacter.HUD` (`local.TheCharacter`)))
      ;[0 0 0] Tady voláme ještě původní akci.
      (`parent.Aktivace` null))))

(fn `UserConstructionScript`
  ;[0 0 0] Nastavujeme sílu výbuchu
  (set `RadialForceComponent.ImpulseStrength` (`self.SilaVybuchu`) (`self.RadialForce`))
  (`ParticleSystemComponent.SetTemplate` (`self.Particle`) (`self.EfektVybuchu`))
  (`parent.UserConstructionScript`))