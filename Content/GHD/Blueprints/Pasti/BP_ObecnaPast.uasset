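; BP_ObecnaPast is a generic trap base Blueprint whose only job is to report that a player character has walked into it.
; The construction script sizes a detection sphere from RadiusDetekce and applies a configurable mesh.
; When the sphere's overlap finds a ThirdPersonCharacter, it passes that character to Aktivace, which currently only prints a debug message.
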(event `self.Sphere.OnComponentBeginOverlap`
  (params (OverlappedComponent :type "PrimitiveComponent Object Reference") (OtherActor :type "Actor Object Reference") (OtherComp :type "PrimitiveComponent Object Reference") (OtherBodyIndex :type Integer) (bFromSweep :type Boolean) (SweepResult :type "HitResult Structure (by ref)"))
  ;[0 0 0] Definice, co má Obecná Past dělat:
  ; (Pouze nám řekne, že někdo prošel)
  ;
  ; Samo o sobě je to "hloupý" blueprint ale umí nám jenom říct, že někdo prošel. To je jeho hlavní úkol.
  (bind _asthird_person_character (cast `/Game/ThirdPersonBP/Blueprints/ThirdPersonCharacter` OtherActor))
  (`self.Aktivace` _asthird_person_character))

(fn `Aktivace`
  (params (Character :type "/Game/ThirdPersonBP/Blueprints/ThirdPersonCharacter Object Reference"))
  (`KismetSystemLibrary.PrintString` "AKTIVACE!"))

(fn `UserConstructionScript`
  (`SphereComponent.SetSphereRadius` (`self.Sphere`) (`self.RadiusDetekce`) true)
  (`StaticMeshComponent.SetStaticMesh` (`self.StaticMesh`) (`self.Mesh`)))