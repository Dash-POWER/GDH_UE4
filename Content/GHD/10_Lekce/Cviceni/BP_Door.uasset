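; BP_Door is a swinging door that opens when a ThirdPersonCharacter enters its collision volume and closes when the character leaves.
; The OpenClose timeline drives the door mesh's yaw, playing forward to open and in reverse to close, with a movement sound for each.
; IsOpen acts as an unlocked flag gating both motions, and ChangeLockState sets it with a sound.
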(event `OpenDoor`
  (if (`self.IsOpen`)
    (bind (_direction _openclose) (`Timeline|OpenClose` :!label _label)
      (:`Update`
        (`SceneComponent.K2_SetRelativeRotation` (`self.Door`) (`KismetMathLibrary.MakeRotator` 0.0 0.0 _openclose) false false)))))

(event `CloseDoor`
  (if (`self.IsOpen`)
    (goto _label :!via `Reverse`)))

(event `self.Collision.OnComponentBeginOverlap`
  (params (OverlappedComponent :type "PrimitiveComponent Object Reference") (OtherActor :type "Actor Object Reference") (OtherComp :type "PrimitiveComponent Object Reference") (OtherBodyIndex :type Integer) (bFromSweep :type Boolean) (SweepResult :type "HitResult Structure (by ref)"))
  (bind _audio (`self.Audio`))
  (cast `/Game/ThirdPersonBP/Blueprints/ThirdPersonCharacter` OtherActor)
  (if (`self.IsOpen`)
    (`self.OpenDoor`)
    ;[1 1 1] Audio
    (`AudioComponent.SetSound` _audio "/Game/GHD/10_Lekce/Cviceni/Sounds/doormove9.doormove9")
    (`AudioComponent.Play` _audio 0.0)))

(event `self.Collision.OnComponentEndOverlap`
  (params (OverlappedComponent :type "PrimitiveComponent Object Reference") (OtherActor :type "Actor Object Reference") (OtherComp :type "PrimitiveComponent Object Reference") (OtherBodyIndex :type Integer))
  (bind _audio (`self.Audio`))
  (cast `/Game/ThirdPersonBP/Blueprints/ThirdPersonCharacter` OtherActor)
  (if (`self.IsOpen`)
    (`self.CloseDoor`)
    ;[1 1 1] Audio
    (`AudioComponent.SetSound` _audio "/Game/GHD/10_Lekce/Cviceni/Sounds/doormove10.doormove10")
    (`AudioComponent.Play` _audio 0.0)))

(event `ChangeLockState`
  (params (State :type Boolean))
  (bind _audio (`self.Audio`))
  ;[1 1 1] Change Open State
  (set `self.IsOpen` State)
  (`AudioComponent.SetSound` _audio "/Game/GHD/10_Lekce/Cviceni/Sounds/doorstop1.doorstop1")
  (`AudioComponent.Play` _audio 0.0))

(fn `UserConstructionScript`)